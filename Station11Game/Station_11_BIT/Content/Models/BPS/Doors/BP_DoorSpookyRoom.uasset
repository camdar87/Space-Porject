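; Sliding double door that the player opens with Interact and that closes itself after a short delay.
; Interact needs IsLookingAtDoor, set outside this graph, and passes a Gate that Box overlaps open only while a Character is inside.
; Timelines lerp both panels along X, with sounds and a green indicator material while open; the open timeline's finish loops back into the close branch.
; The prompt widget logic is disconnected.
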(event `InputAction|Interact` :consume false
  (params (Key :type "Key Structure"))
  (bind _returnvalue (`self.K2_GetActorLocation`))
  ;[1 1 1] Checks if looking at door
  (:`Pressed`
    (`KismetSystemLibrary.Delay` 0.2)
    (if (`self.IsLookingAtDoor?`)
      (set `self.IsLookingAtDoor?` false)
      (`/Engine/EditorBlueprintResources/StandardMacros.Gate` true :!label _label
        (:`Exit`
          (if (`self.IsDoorClosed?`) :!label _label_2
            ;[1 1 1] Open
            (`|ExecutionSequence`
              (:`then_0`
                (bind (_direction _open_close) (`Timeline|Door` :!via `PlayFromStart`)
                  (:`Update`
                    (`SceneComponent.K2_SetRelativeLocation` (`self.Door2`) (`KismetMathLibrary.MakeVector` (`KismetMathLibrary.Lerp` (`self.CloseDoor2`) (`self.OpenDoor2`) _open_close)) false false)
                    (`SceneComponent.K2_SetRelativeLocation` (`self.Door1`) (`KismetMathLibrary.MakeVector` (`KismetMathLibrary.Lerp` (`self.CloseDoor1`) (`self.OpenDoor1`) _open_close)) false false))
                  (:`Finished`
                    (set `self.IsDoorClosed?` false)
                    (goto _label_2))))
              (:`then_1`
                (`GameplayStatics.SpawnSoundAtLocation` "/Game/Audio/CUE_Granted.CUE_Granted" _returnvalue (struct) 0.7 1.0 0.0 null null)
                (`GameplayStatics.SpawnSoundAtLocation` "/Game/Audio/CUE_DoorOpen.CUE_DoorOpen" _returnvalue (struct) 0.7 1.0 0.0 null null))
              (:`then_2`
                (`PrimitiveComponent.SetMaterial` (`self.Plane2`) 0 "/Game/Materials/MAT_LIGHT_GREEN.MAT_LIGHT_GREEN")))
            (else
              ;[1 1 1] Close
              (`KismetSystemLibrary.Delay` 2.0)
              (`|ExecutionSequence`
                (:`then_0`
                  (bind (_direction_2 _open_close_2) (`Timeline|Timeline_0` :!via `ReverseFromEnd`)
                    (:`Update`
                      (`SceneComponent.K2_SetRelativeLocation` (`self.Door2`) (`KismetMathLibrary.MakeVector` (`KismetMathLibrary.Lerp` (`self.CloseDoor2`) (`self.OpenDoor2`) _open_close_2)) false false)
                      (`SceneComponent.K2_SetRelativeLocation` (`self.Door1`) (`KismetMathLibrary.MakeVector` (`KismetMathLibrary.Lerp` (`self.CloseDoor1`) (`self.OpenDoor1`) _open_close_2)) false false))
                    (:`Finished`
                      (set `self.IsDoorClosed?` true)
                      (`PrimitiveComponent.SetMaterial` (`self.Plane2`) 0 "/Game/Materials/LIGHT.LIGHT"))))
                (:`then_1`
                  (`GameplayStatics.SpawnSoundAtLocation` "/Game/Audio/CUE_DoorOpen.CUE_DoorOpen" _returnvalue (struct) 0.3 1.0 0.0 null null))))))))))

(event `self.Box.OnComponentBeginOverlap`
  (params (OverlappedComponent :type "PrimitiveComponent Object Reference") (OtherActor :type "Actor Object Reference") (OtherComp :type "PrimitiveComponent Object Reference") (OtherBodyIndex :type Integer) (bFromSweep :type Boolean) (SweepResult :type "HitResult Structure (by ref)"))
  ;[1 1 1] checks for close enough
  (cast `Character` OtherActor)
  (goto _label :!via `Open`))

(event `self.Box.OnComponentEndOverlap`
  (params (OverlappedComponent :type "PrimitiveComponent Object Reference") (OtherActor :type "Actor Object Reference") (OtherComp :type "PrimitiveComponent Object Reference") (OtherBodyIndex :type Integer))
  ;[1 1 1] checks for close enough
  (cast `Character` OtherActor)
  (goto _label :!via `Close`))

(event `self.ReceiveBeginPlay`
  ;[1 1 1] Enable use of interact
  (`self.EnableInput` (`GameplayStatics.GetPlayerController` 0))
  (set `self.IsPressed` false))

(fn `UserConstructionScript`)