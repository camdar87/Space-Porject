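; Door actor that swings its Door component between zero rotation and a 90-degree turn.
; While IsPlaying is set, Tick calls OpenClose, which eases the relative rotation with RInterpTo toward the target chosen by IsClosed.
; Near the target it flips IsClosed, which becomes true at 90 degrees, and clears IsPlaying.
; Open and Close are empty stubs, and nothing here starts playback.
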(event `self.ReceiveTick`
  (params (DeltaSeconds :type "Float (single-precision)"))
  (if (`self.isPlaying`)
    (`self.OpenClose` DeltaSeconds)))

(fn `Close`)

(fn `Open`)

(fn `OpenClose`
  (params (DeltaTime :type "Float (double-precision)"))
  (bind _door (`self.Door`))
  (bind _returnvalue (`KismetMathLibrary.RInterpTo` (`SceneComponent.RelativeRotation` (`self.Door`)) (struct :`Yaw` 90.0) DeltaTime 1.0))
  (bind _returnvalue_2 (`KismetMathLibrary.RInterpTo` (`SceneComponent.RelativeRotation` (`self.Door`)) (struct) DeltaTime 1.0))
  (if (`self.isClosed`)
    (`SceneComponent.K2_SetRelativeRotation` _door _returnvalue_2 false false)
    (if (== _returnvalue_2 (`SceneComponent.RelativeRotation` _door) :`ErrorTolerance` 0.1)
      (set `self.isClosed` false)
      (set `self.isPlaying` false :!label _label))
    (else
      (`SceneComponent.K2_SetRelativeRotation` _door _returnvalue false false)
      (if (== _returnvalue (`SceneComponent.RelativeRotation` _door) :`ErrorTolerance` 0.1)
        (set `self.isClosed` true)
        (goto _label)))))

(fn `UserConstructionScript`)