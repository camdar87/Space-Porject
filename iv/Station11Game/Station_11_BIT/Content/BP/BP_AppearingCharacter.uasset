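; BP_AppearingCharacter is a character figure that briefly appears when something overlaps its trigger box.
; Nested FlipFlops on the box's begin overlap gate the effect to the first of every four overlaps, with no filter on the overlapping actor.
; That overlap shows the skeletal mesh for a short delay and then hides it, while the other three just hide it.
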(event `self.Box.OnComponentBeginOverlap`
  (params (OverlappedComponent :type "PrimitiveComponent Object Reference") (OtherActor :type "Actor Object Reference") (OtherComp :type "PrimitiveComponent Object Reference") (OtherBodyIndex :type Integer) (bFromSweep :type Boolean) (SweepResult :type "HitResult Structure (by ref)"))
  (`/Engine/EditorBlueprintResources/StandardMacros.FlipFlop`
    (:`A`
      (`/Engine/EditorBlueprintResources/StandardMacros.FlipFlop`
        (:`A`
          (`SceneComponent.SetVisibility` (`self.SkeletalMesh`) true false)
          (`KismetSystemLibrary.Delay` 2.0)
          (`SceneComponent.SetVisibility` (`self.SkeletalMesh`) false false))
        (:`B`
          (`SceneComponent.SetVisibility` (`self.SkeletalMesh`) false false))))
    (:`B`
      (`SceneComponent.SetVisibility` (`self.SkeletalMesh`) false false))))

(fn `UserConstructionScript`)